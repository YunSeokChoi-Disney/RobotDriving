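; Base robot character Blueprint that feeds a state widget, reports to a relay station and opens a test connection to a local message server.
; BeginPlay fills the widget for its data-table row name and connects, printing replies.
; Tick sends itself and its location to the RegisterGameState target station.
; An evade command sets a collision-risk Blackboard flag, and UpdateRobotStateUI derives clamped acceleration from velocity change for the widget.
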(event `self.ReceiveBeginPlay`
  ; 메인로직(Project1)
  (`|ExecutionSequence`
    (:`then_0`
      (bind _asrobot_state_widget (cast `/Game/Data/RobotState_Widget` (`WidgetComponent.GetUserWidgetObject` (`self.Widget`))))
      ;; 여기서 Row Name바꾸면 로봇 종류 바뀜
      (`/Game/Data/RobotState_Widget.UpdateRobotInfo` _asrobot_state_widget (`self.MaxSpeed`) (`self.Acceleration`) (`self.MyRowName`)))
    (:`then_1`
      ;; 테스트용
      (add `self.OnMessageReceived` (delegate `OnRobotMessageRespons`))
      (bind _returnvalue (`self.ConnectToServer` "127.0.0.1" 8888))
      (if _returnvalue
        (`KismetSystemLibrary.PrintString` "서버 연결 성공")
        (else
          (`KismetSystemLibrary.PrintString` "연결 실패"))))))

(event `OnRobotMessageRespons` :!signature `self.OnMessageReceived`
  (params (RobotClientID :type Integer) (Message :type String))
  ; 메인로직(Project1)
  ;; 테스트용
  (`KismetSystemLibrary.PrintString` Message))

(event `self.OnReceiveEvadeCommand`
  (bind _returnvalue (`AIBlueprintHelperLibrary.GetAIController` null))
  ; 메인로직(Project1)
  (`/Engine/EditorBlueprintResources/StandardMacros.IsValid` _returnvalue
    (:`Is Valid`
      (`BlackboardComponent.SetValueAsBool` (`AIBlueprintHelperLibrary.GetBlackboard` _returnvalue) "bIsCollisionRisk" true))))

(event `Key|One`
  (params (Key :type "Key Structure"))
  ; 메인로직(Project1)
  ;; 테스트용
  (:`Pressed`
    (`self.SendMessageToServer` "Hello Python! I am Unreal Robot.")))

(event `self.ReceiveTick`
  (params (DeltaSeconds :type "Float (single-precision)"))
  ; 메인로직(Project1)
  ;; 중계소 방식 로직 구현 중
  (bind _asregister_game_state (cast `/Game/BluePrints/RobotStation/RegisterGameState` (`GameplayStatics.GetGameState`))
    (:`then`
      (bind _targetstation (`/Game/BluePrints/RobotStation/RegisterGameState.TargetStation` _asregister_game_state))
      (`/Engine/EditorBlueprintResources/StandardMacros.IsValid` _targetstation
        (:`Is Valid`
          (bind _output_get (set `self.ConnectedStation` _targetstation))
          (`/Engine/EditorBlueprintResources/StandardMacros.IsValid` _output_get
            (:`Is Valid`
              (`/Game/BluePrints/RobotStation/BP_RobotStation.ReceiveRobotData` _output_get self (`self.K2_GetActorLocation`) (0.0 0.0 0.0) "" 0))
            (:`Is Not Valid`
              (`KismetSystemLibrary.PrintString` "ConnectedStation Failed!!" true true (struct :`R` 1.0 :`G` 0.081243 :`A` 1.0) 9999.0))))
        (:`Is Not Valid`
          (`KismetSystemLibrary.PrintString` "Target Station is Empty"))))
    (:`CastFailed`
      (`KismetSystemLibrary.PrintString` "RegisterGameState Cast Faliled!!"))))

(fn `UpdateRobotStateUI`
  (params (TargetWidget :type "/Game/Data/RobotState_Widget Object Reference"))
  (bind _returnvalue (`self.GetVelocity`))
  (`/Engine/EditorBlueprintResources/StandardMacros.IsValid` TargetWidget
    (:`Is Valid`
      (cast `/Game/Data/RobotState_Widget` (`WidgetComponent.GetUserWidgetObject` (`self.Widget`)))
      ; 로봇 위젯의 상태 정보 업데이트  하는 함수
      (`/Game/Data/RobotState_Widget.UpdateRobotInfo` TargetWidget (`KismetMathLibrary.VSize` _returnvalue) (`KismetMathLibrary.FClamp` (/ (- (`KismetMathLibrary.VSize` (`self.GetVelocity`)) (`KismetMathLibrary.VSize` (`self.PreviousVelocity`))) (`GameplayStatics.GetWorldDeltaSeconds`)) -300.0 300.0) (`self.MyRowName`))
      ; 이전 속도 업데이트
      (set `self.PreviousVelocity` _returnvalue))
    (:`Is Not Valid`
      ; Widget정보 유효한지 디버깅
      (`KismetSystemLibrary.PrintString` "Hello"))))

(fn `UserConstructionScript`)