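; Robot station that registers itself as TargetStation on the RegisterGameState and collects position data from robots.
; ReceiveRobotData stores each robot's current and target locations in a map, prints the sender, then checks only the first key.
; CheckandControlRobot tests proximity to a different robot or draws a debug line for the sender itself.
; The proximity branch is empty and the speed-stop logic is unconnected, so no robot is controlled yet.
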(event `self.ReceiveBeginPlay`
  (bind _asregister_game_state (cast `/Game/BluePrints/RobotStation/RegisterGameState` (`GameplayStatics.GetGameState`))
    (:`then`
      (set `/Game/BluePrints/RobotStation/RegisterGameState.TargetStation` self _asregister_game_state))
    (:`CastFailed`
      (`KismetSystemLibrary.PrintString` "Gamestate Cast Failed!!"))))

(fn `CheckandControlRobot`
  (params (SelfRobot :type "/Game/BluePrints/BP_Robot_base Object Reference") (TargetMap :type "Map of Object Object Reference to /Game/Data/Struct/ST_RobotData Structure (by ref)") (Key :type "Object Object Reference (by ref)") (B :type "Object Object Reference") (A :type "Object Object Reference") (LineStart :type "Vector Structure") (V1 :type "Vector Structure"))
  (bind (_value _returnvalue) (`BlueprintMapLibrary.Map_Find` TargetMap Key))
  (bind _currentlocation (break `/Game/Data/Struct/ST_RobotData` _value))
  (if (!= A B)
    (if _returnvalue
      (if (< (`KismetMathLibrary.Vector_Distance` V1 _currentlocation) 300.0)
        _))
    (else
      (`KismetSystemLibrary.DrawDebugLine` LineStart _currentlocation (struct :`G` 1.0 :`A` 1.0) 0.1 1.0))))

(fn `ReceiveRobotData`
  (params (RobotRef :type "Actor Object Reference") (CurrentLoc :type "Vector Structure") (TargetLoc :type "Vector Structure"))
  (`BlueprintMapLibrary.Map_Add` (`self.RobotDataMap`) RobotRef (make `/Game/Data/Struct/ST_RobotData` CurrentLoc TargetLoc))
  (`KismetSystemLibrary.PrintString` (`KismetStringLibrary.Concat_StrStr` "수신로봇: " (`KismetSystemLibrary.GetDisplayName` RobotRef)))
  (bind _keys (`BlueprintMapLibrary.Map_Keys` (`self.RobotDataMap`)))
  (for _array_element _keys
    (`self.CheckandControlRobot` null (`self.RobotDataMap`) _array_element _array_element RobotRef CurrentLoc CurrentLoc)
    (break)))

(fn `UserConstructionScript`)