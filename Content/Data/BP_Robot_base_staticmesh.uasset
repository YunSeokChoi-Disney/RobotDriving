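; Base robot Blueprint that shows its spec and movement state in an on-screen RobotState_Widget.
; BeginPlay looks up MyRowName in DT_RobotLibraries, passes name, ID, sensor and movement limits to a new widget, and adds it to the viewport.
; UpdateRobotStateUI sends current speed and acceleration magnitudes to that widget, but nothing here calls it.
; Logic applying table speed to CharacterMovement is disconnected, and NewFunction is empty.
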(event `self.ReceiveBeginPlay`
  ; 메인로직
  (bind _returnvalue (`|GetDataTableRow` "/Game/Data/DataTable/DT_RobotLibraries.DT_RobotLibraries" (`self.MyRowName`))
    (:`then`
      (bind _returnvalue_2 (`|CreateWidget` "/Game/Data/RobotState_Widget.RobotState_Widget_C" null (make `/Game/Data/Struct/ST_RobotLibraries` (break `/Game/Data/Struct/ST_RobotLibraries` _returnvalue) (`.Robot_ID_3_5C0497E24E10086CCBDD9AA7748F0570` (break `/Game/Data/Struct/ST_RobotLibraries` _returnvalue)) (`.SensorRange_9_1D81A3CC4680596E870AE4B216473736` (break `/Game/Data/Struct/ST_RobotLibraries` _returnvalue)) (`.SensorFoV_12_33EE212A4FA40607D0FA04B92125A5EB` (break `/Game/Data/Struct/ST_RobotLibraries` _returnvalue)) (`.MaxSpeed_14_FE56CFF747F5C1EF58D086AF348B91C6` (break `/Game/Data/Struct/ST_RobotLibraries` _returnvalue)) (`.Acceleration_17_3CD6DA01443AECF9BC2DCFAC06735188` (break `/Game/Data/Struct/ST_RobotLibraries` _returnvalue)))))
      (bind _output_get (set `self.RobotStateWidget` _returnvalue_2))
      (`UserWidget.AddToViewport` _output_get 0))))

(fn `NewFunction`
  (params (Yaw :type "Float (single-precision)")))

(fn `UpdateRobotStateUI`
  (`/Game/Data/RobotState_Widget.UpdateRobotInfo` (`self.RobotStateWidget`) (`KismetMathLibrary.VSize` (`self.GetVelocity`)) (`KismetMathLibrary.VSize` (`CharacterMovementComponent.GetCurrentAcceleration` (`self.CharacterMovement`)))))

(fn `UserConstructionScript`)